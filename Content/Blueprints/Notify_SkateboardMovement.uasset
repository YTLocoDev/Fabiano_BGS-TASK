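; Animation notify that syncs skateboard movement with animation frames, applying either a push or a jump to the owning Character.
; A skate-state enum selects the action and also sets the notify's display name.
; On trigger it casts the mesh owner to Character, then either launches it along its forward vector with an additive impulse or calls Jump.
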(fn `GetNotifyName`
  (returns (ReturnValue :type String))
  (return (select `/Game/Blueprints/Enums/E_CharacterSkateboardMovementStates` (`self.CharacterSkateStates`) :`NewEnumerator0` "Jump Event" :`NewEnumerator1` "Push Event")))

(fn `Launch Character`
  (params (Target :type "Character Object Reference") (`Launch Force` :type "Float (single-precision)"))
  (`Character.LaunchCharacter` Target (* (`Actor.GetActorForwardVector` Target) `Launch Force`) false false))

(fn `Received_Notify`
  (params (MeshComp :type "SkeletalMeshComponent Object Reference") (Animation :type "AnimSequenceBase Object Reference") (EventReference :type "AnimNotifyEventReference Structure (by ref)"))
  (returns (ReturnValue :type Boolean))
  (locals (Character :type "Character Object Reference"))
  (bind _ascharacter (cast `Character` (`ActorComponent.GetOwner` MeshComp)))
  (set `local.Character` _ascharacter)
  ;[0.07812 0.07812 0.07812] Push Action: Add a notify state within the animation to align the character's movement with the animation frames.
  (if (`|EnumEquality` (`self.CharacterSkateStates`) "NewEnumerator1")
    (`self.Launch Character` (`local.Character`) 500.0)
    (return true)
    (else
      ;[0.07812 0.07812 0.07812] Jump Event: Add a notification within the animation to synchronize the character's jump with the animation frames.
      (if (`|EnumEquality` (`self.CharacterSkateStates`) "NewEnumerator0")
        (`Character.Jump` (`local.Character`))
        (return true)))))